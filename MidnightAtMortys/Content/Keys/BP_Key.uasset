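; BP_Key is an interactable key that unlocks the playground door.
; Its Trigger shows a widget when BP_Player begins overlapping and hides it when any overlap ends.
; On Interact, it clears IsLocked on BP_PlaygroundDoor, destroys itself and turns off BP_KeyLight, finding both other actors through GetActorOfClass rather than stored references.
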(event OnComponentBeginOverlap(Trigger)
  (params (OverlappedComponent :type Primitive%20Component%20Object%20Reference) (OtherActor :type Actor%20Object%20Reference) (OtherComp :type Primitive%20Component%20Object%20Reference) (OtherBodyIndex :type Integer) (bFromSweep :type Boolean) (SweepResult :type Hit%20Result%20Structure%20%28by%20ref%29))
  (Utilities|Casting|CastToBP_Player OtherActor)
  (Rendering|SetVisibility (Variables|Default|GetWidget) true false))

(event OnComponentEndOverlap(Trigger)
  (params (OverlappedComponent :type Primitive%20Component%20Object%20Reference) (OtherActor :type Actor%20Object%20Reference) (OtherComp :type Primitive%20Component%20Object%20Reference) (OtherBodyIndex :type Integer))
  (Rendering|SetVisibility (Variables|Default|GetWidget) false false))

(event EventBeginPlay)

(event Collision|EventActorBeginOverlap
  (params (OtherActor :type Actor%20Object%20Reference)))

(event EventTick
  (params (DeltaSeconds :type Float%20%28single-precision%29)))

(event EventInteract
  (bind _returnvalue (Actor|GetActorOfClass "/Game/Door/BP_PlaygroundDoor.BP_PlaygroundDoor_C"))
  (Variables|/Game/Door/BP_PlaygroundDoor.BP_PlaygroundDoor_C|SetisLocked _returnvalue false)
  (Actor|DestroyActor)
  (bind _returnvalue_2 (Actor|GetActorOfClass "/Game/CeilingLight/BP_KeyLight.BP_KeyLight_C"))
  (Default|TurnOff _returnvalue_2))

(fn ConstructionScript)