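; BP_NoteBoard is a board actor that displays the notes the player has collected.
; Every Tick, a Sequence casts the player character to BP_Player and checks a separate flag for each of four notes.
; Each set flag makes its matching note component visible; nothing in this Blueprint hides one again.
; The state is polled each frame rather than driven by events.
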(event Collision|EventActorBeginOverlap
  (params (OtherActor :type Actor%20Object%20Reference)))

(event EventTick
  (params (DeltaSeconds :type Float%20%28single-precision%29))
  (bind _returnvalue (Game|GetPlayerCharacter 0))
  (Utilities|FlowControl|Sequence
    (:then_0
      (bind _asbp_player (Utilities|Casting|CastToBP_Player _returnvalue))
      (if (Variables|/Game/Player/BP_Player.BP_Player_C|GetHasNote1 _asbp_player)
        (Rendering|SetVisibility (Variables|Default|GetNote1) true false)))
    (:then_1
      (bind _asbp_player_2 (Utilities|Casting|CastToBP_Player _returnvalue))
      (if (Variables|/Game/Player/BP_Player.BP_Player_C|GetHasNote2 _asbp_player_2)
        (Rendering|SetVisibility (Variables|Default|GetNote2) true false)))
    (:then_2
      (bind _asbp_player_3 (Utilities|Casting|CastToBP_Player _returnvalue))
      (if (Variables|/Game/Player/BP_Player.BP_Player_C|GetHasNote3 _asbp_player_3)
        (Rendering|SetVisibility (Variables|Default|GetNote3) true false)))
    (:then_3
      (bind _asbp_player_4 (Utilities|Casting|CastToBP_Player _returnvalue))
      (if (Variables|/Game/Player/BP_Player.BP_Player_C|GetHasNote4 _asbp_player_4)
        (Rendering|SetVisibility (Variables|Default|GetNote4) true false)))))

(event EventBeginPlay)

(fn ConstructionScript)