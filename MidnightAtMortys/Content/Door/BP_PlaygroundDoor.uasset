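; BP_PlaygroundDoor is an interactable hinged door that opens and closes on Interact unless locked.
; Separate open and close timelines drive the Hinge yaw, with the close timeline played in reverse from its end.
; DoorFrame collision is disabled while opening and restored while closing, and a sound plays only on opening.
; The Interactable flag blocks further interaction until the running timeline finishes.
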(event EventBeginPlay)

(event Collision|EventActorBeginOverlap
  (params (OtherActor :type Actor%20Object%20Reference)))

(event EventTick
  (params (DeltaSeconds :type Float%20%28single-precision%29)))

(event EventInteract
  (if (not (Variables|Default|GetisLocked))
    (if (Variables|Default|GetdoorIsOpen)
      (if (Variables|Default|Getinteractable)
        (bind _doorclose (Timeline|DoorClose ReverseFromEnd)
          (:Update
            (Transformation|SetRelativeRotation (Variables|Default|GetHinge) (Math|Rotator|MakeRotator 0.0 0.0 _doorclose) false false)
            (Variables|Default|SetdoorIsOpen false)
            (Collision|SetCollisionEnabled (Variables|Default|GetDoorFrame) "QueryAndPhysics")
            (Variables|Default|Setinteractable false))
          (:Finished
            (Variables|Default|Setinteractable true))))
      (elif (Variables|Default|Getinteractable)
        (Audio|PlaySoundatLocation "/Game/Door/DoorSounds/DoorOpen.DoorOpen" (Transformation|GetWorldLocation (Variables|Default|GetDoorFrame)) "0, 0, 0" 0.2 1.0 0.25 0 0 0 0)
        (bind _dooropen (Timeline|DoorOpen PlayFromStart)
          (:Update
            (Transformation|SetRelativeRotation (Variables|Default|GetHinge) (Math|Rotator|MakeRotator 0.0 0.0 _dooropen) false false)
            (Variables|Default|SetdoorIsOpen true)
            (Collision|SetCollisionEnabled (Variables|Default|GetDoorFrame) "NoCollision")
            (Variables|Default|Setinteractable false))
          (:Finished
            (Variables|Default|Setinteractable true)))))))

(fn ConstructionScript)