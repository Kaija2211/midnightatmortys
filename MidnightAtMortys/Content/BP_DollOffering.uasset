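; BP_DollOffering is an interactable offering spot where the player places dolls and sets the flag for unlocking the main door.
; A box overlap shows or hides the prompt widget for BP_Player until the offering is made.
; Interact marks it as offered, reveals the Morty, bear and deer meshes, hides the prompt, calls Message on the player, then sets UnlockMainDoor.
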(event OnComponentBeginOverlap(Box)
  (params (OverlappedComponent :type Primitive%20Component%20Object%20Reference) (OtherActor :type Actor%20Object%20Reference) (OtherComp :type Primitive%20Component%20Object%20Reference) (OtherBodyIndex :type Integer) (bFromSweep :type Boolean) (SweepResult :type Hit%20Result%20Structure%20%28by%20ref%29))
  (Utilities|Casting|CastToBP_Player OtherActor)
  (if (not (Variables|Default|GetOffered))
    (Rendering|SetVisibility (Variables|Default|GetWidget) true false)))

(event OnComponentEndOverlap(Box)
  (params (OverlappedComponent :type Primitive%20Component%20Object%20Reference) (OtherActor :type Actor%20Object%20Reference) (OtherComp :type Primitive%20Component%20Object%20Reference) (OtherBodyIndex :type Integer))
  (Utilities|Casting|CastToBP_Player OtherActor)
  (if (not (Variables|Default|GetOffered))
    (Rendering|SetVisibility (Variables|Default|GetWidget) false false)))

(event EventInteract
  (Utilities|FlowControl|Sequence
    (:then_0
      (Variables|Default|SetOffered true)
      (Rendering|SetVisibility (Variables|Default|GetMortyMesh) true false)
      (Rendering|SetVisibility (Variables|Default|GetBearMesh) true false)
      (Rendering|SetVisibility (Variables|Default|GetDeerMesh) true false)
      (Rendering|SetVisibility (Variables|Default|GetWidget) false false)
      (bind _returnvalue (Actor|GetActorOfClass "/Game/Player/BP_Player.BP_Player_C"))
      (Default|Message _returnvalue))
    (:then_1
      (Variables|Default|SetUnlockMainDoor true))))

(fn ConstructionScript)