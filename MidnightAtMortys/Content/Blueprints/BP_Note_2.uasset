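; BP_Note_2 is the second collectible note, picked up through its Interact event.
; Interact finds BP_NoteBoard to show note two, destroys the note actor, then turns off BP_Clue2Light, locating both actors by class lookup.
; An unconnected box-overlap branch that would set HasNote2 on BP_Player never runs, and the remaining events are empty.
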(event Custom|CustomEvent
  ;[1 1 1] Change this to an Interact event
)

(event EventBeginPlay)

(event EventTick
  (params (DeltaSeconds :type Float%20%28single-precision%29)))

(event Collision|EventActorBeginOverlap
  (params (OtherActor :type Actor%20Object%20Reference)))

(event EventInteract
  (bind _returnvalue (Actor|GetActorOfClass "/Game/Blueprints/BP_NoteBoard.BP_NoteBoard_C"))
  (Default|NoteTwoVisible _returnvalue)
  (Actor|DestroyActor)
  (bind _returnvalue_2 (Actor|GetActorOfClass "/Game/CeilingLight/BP_Clue2Light.BP_Clue2Light_C"))
  (Default|TurnOff _returnvalue_2))

(fn ConstructionScript)