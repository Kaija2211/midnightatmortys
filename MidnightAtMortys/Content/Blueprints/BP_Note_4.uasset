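; BP_Note_4 is the fourth collectible note, picked up through its Interact event.
; A Box overlap shows the prompt Widget for BP_Player and hides it on any end overlap.
; Interact reveals note four on BP_NoteBoard, destroys the note, then switches BP_Clue4Light off and BP_StageLights on, finding each via GetActorOfClass.
; An unconnected older pickup path that sets HasNote4 on the player never runs.
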(event OnComponentBeginOverlap(Box)
  (params (OverlappedComponent :type Primitive%20Component%20Object%20Reference) (OtherActor :type Actor%20Object%20Reference) (OtherComp :type Primitive%20Component%20Object%20Reference) (OtherBodyIndex :type Integer) (bFromSweep :type Boolean) (SweepResult :type Hit%20Result%20Structure%20%28by%20ref%29))
  (Utilities|Casting|CastToBP_Player OtherActor)
  (Rendering|SetVisibility (Variables|Default|GetWidget) true false))

(event OnComponentEndOverlap(Box)
  (params (OverlappedComponent :type Primitive%20Component%20Object%20Reference) (OtherActor :type Actor%20Object%20Reference) (OtherComp :type Primitive%20Component%20Object%20Reference) (OtherBodyIndex :type Integer))
  (Rendering|SetVisibility (Variables|Default|GetWidget) false false))

(event Custom|CustomEvent
  ;[1 1 1] Change this to an Interact event
)

(event EventBeginPlay)

(event EventTick
  (params (DeltaSeconds :type Float%20%28single-precision%29)))

(event Collision|EventActorBeginOverlap
  (params (OtherActor :type Actor%20Object%20Reference)))

(event EventInteract
  (bind _returnvalue (Actor|GetActorOfClass "/Game/Blueprints/BP_NoteBoard.BP_NoteBoard_C"))
  (Default|NoteFourVisible _returnvalue)
  (Actor|DestroyActor)
  (bind _returnvalue_2 (Actor|GetActorOfClass "/Game/CeilingLight/BP_Clue4Light.BP_Clue4Light_C"))
  (Default|TurnOff _returnvalue_2)
  (bind _returnvalue_3 (Actor|GetActorOfClass "/Game/BP_StageLights.BP_StageLights_C"))
  (Default|Turnon _returnvalue_3))

(fn ConstructionScript)